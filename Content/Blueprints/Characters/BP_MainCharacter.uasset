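; Main character Blueprint that drives Niagara effects for its abilities, including a drawing ability.
; Each Tick feeds AbilityEffectComponent a SpawnPosition a fixed distance from the actor along the control rotation's forward vector, so the effect follows the aim.
; SpawnFX spawns a given Niagara system, if valid, at the world location of DrawingAbilityComponent's spline.
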(event EventBeginPlay)

(event EventTick
  (params (DeltaSeconds :type Float%20%28single-precision%29))
  (Class|NiagaraComponent|SetVariablePosition (Variables|Default|GetAbilityEffectComponent) "SpawnPosition" (+ (Transformation|GetActorLocation) (* (Math|Vector|GetForwardVector (Pawn|GetControlRotation :!class /Script/Engine.Pawn)) 1.5e+02))))

(fn ConstructionScript)

(fn SpawnFX
  (params (VFX%20to%20Spawn :type Niagara%20System%20Object%20Reference))
  (Utilities|IsValid VFX%20to%20Spawn
    (:Is%20Valid
      (Niagara|SpawnSystematLocation VFX%20to%20Spawn (Transformation|GetWorldLocation (Variables|/Script/straw.DrawingAbilityComponent|GetSplineComponent (Variables|Default|GetDrawingAbilityComponent)))))))
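; Main character Blueprint that adds ledge grabbing, hanging, climb-up and drop to jumping.
; Jump sphere-traces for a ledge, then HangOnLedge aligns the capsule in Flying mode, snapping when airborne or playing a motion-warped montage from the ground.
; While hanging, looping timers trace hand IK targets and foot surfaces for braced or free hang.
; W climbs via a warped montage when clearance allows; S drops into Falling.
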(event Custom|LedgeClimbInput
  (bind _charactermovement (Variables|Character|GetCharacterMovement))
  (bind _returnvalue (AI|Components|NavMovement|IsFalling _charactermovement))
  ;[1 1 1] Do ledge or jump
  (if (not (Variables|Default|GetIsOnLedge))
    (bind (_ledgedetected _ledgelocation _ledgenormal) (CallFunction|TraceLedge (Math|Float|SelectFloat 0.0 25.0 _returnvalue) 4e+01 (Math|Float|SelectFloat 25.0 1e+01 _returnvalue) "ForDuration"))
    (if _ledgedetected
      (Utilities|HangonLedge _ledgelocation _ledgenormal)
      (else
        (Character|Jump)))))

(event Custom|CheckIfLedgeHasSurface
  (bind _returnvalue (Transformation|GetActorForwardVector))
  (bind _skeletalmesh (Variables|Default|GetSkeletalMesh))
  (bind _returnvalue_2 (Transformation|GetWorldLocation _skeletalmesh))
  (bind _returnvalue_3 (* _returnvalue 8e+01))
  (bind _returnvalue_4 (+ _returnvalue_2 "25.000000,0.000000,70.000000"))
  (bind _returnvalue_5 (+ _returnvalue_2 "-25.000000,0.000000,70.000000"))
  ;[1 1 1] Check if the ledge has a surface so each foot can either be placed on the ledge or hanging
  (Utilities|FlowControl|Sequence
    (:then_0
      (bind _returnvalue_6 (Collision|LineTraceByChannel _returnvalue_4 (+ _returnvalue_4 _returnvalue_3) "TraceTypeQuery1" false 0 "None"))
      (Variables|Default|SetLedgeHasSurface_L _returnvalue_6))
    (:then_1
      (bind _returnvalue_7 (Collision|LineTraceByChannel _returnvalue_5 (+ _returnvalue_5 _returnvalue_3) "TraceTypeQuery1" false 0 "None"))
      (Variables|Default|SetLedgeHasSurface_R _returnvalue_7))))

(event Custom|LedgeHandIK
  ;[1 1 1] Find ledge hand locations
  (bind _ishit (CallFunction|FindLedgeHandIKLocation (Variables|Default|GetHandIKLocation_L) -17.0 "ForOneFrame"))
  (bind _ishit_2 (CallFunction|FindLedgeHandIKLocation (Variables|Default|GetHandIKLocation_R) 17.0 "ForOneFrame"))
  (if (not (and _ishit _ishit_2))
    (Variables|Default|SetHandIKTargetAlpha 0.0)))

(event EventBeginPlay)

(event EventTick
  (params (DeltaSeconds :type Float%20%28single-precision%29)))

(event Input|ActionEvents|InputActionJump
  (params (Key :type Key%20Structure :default "None"))
  (:Pressed
    (CallFunction|LedgeClimbInput)))

(event Input|KeyboardEvents|W
  (params (Key :type Key%20Structure :default "None"))
  (bind _returnvalue (Transformation|GetActorLocation))
  (bind _returnvalue_2 (Transformation|GetActorForwardVector))
  (bind _ledgeikhandle (Variables|Default|GetLedgeIKHandle))
  (bind _capsulecomponent (Variables|Default|GetCapsuleComponent))
  (bind _capsulecomponent_2 (Variables|Default|GetCapsuleComponent))
  (bind _returnvalue_3 (Components|Capsule|GetScaledCapsuleHalfHeight _capsulecomponent))
  (bind _returnvalue_4 (* _returnvalue_2 8e+01))
  (bind _returnvalue_5 (+ _returnvalue _returnvalue_4))
  (bind _returnvalue_6 (+ _returnvalue_3 55.0))
  (bind _returnvalue_7 (+ _returnvalue_5 (Math|Vector|MakeVector 0.0 0.0 _returnvalue_6)))
  ;[1 1 1] Climb
  (:Pressed
    (if (Variables|Default|GetIsOnLedge)
      (bind _returnvalue_8 (Collision|CapsuleTraceByChannel _returnvalue_7 _returnvalue_7 17.8 35.0 "TraceTypeQuery1" false 0 "ForDuration"))
      (if (not _returnvalue_8)
        (Variables|Default|SetIsOnLedge false)
        (Collision|SetActorEnableCollision false)
        (Utilities|FlowControl|Sequence
          (:then_0
            (bind _outhit (Collision|LineTraceByChannel _returnvalue_7 (- _returnvalue_7 "0.000000,0.000000,50.000000") "TraceTypeQuery1" false 0 "None"))
            (Utilities|FlowControl|Sequence
              (:then_0
                (Components|MoveComponentTo _capsulecomponent_2 (+ (Transformation|GetWorldLocation _capsulecomponent_2) "0.000000,0.000000,60.000000") (Transformation|GetWorldRotation _capsulecomponent_2) false false 0.2 true))
              (:then_1
                (if (Utilities|Time|IsValidTimerHandle _ledgeikhandle)
                  (Utilities|Time|ClearandInvalidateTimerbyHandle _ledgeikhandle))
                (Class|MotionWarpingComponent|AddorUpdateWarpTarget (Variables|Default|GetMotionWarping) (Utilities|Struct|MakeMotionWarpingTarget "ClimbPosition" (+ (.Location (Collision|BreakHitResult _outhit)) "0.000000,0.000000,10.000000") (Transformation|GetActorRotation)))
                (Variables|Default|SetbCanMove true)
                (Animation|Montage|PlayMontage (Variables|Character|GetMesh) "/Game/Animation_Prepare/LedgeClimbing/EnterExit/BracedHangToCrouch_Montage.BracedHangToCrouch_Montage"
                  (:OnBlendOut
                    (Collision|SetActorEnableCollision true))))
              (:then_2
                (Utilities|Time|ClearTimerbyFunctionName 0 "CheckIfLedgeHasSurface"))))
          (:then_1
            (Utilities|FlowControl|Delay 0.8)
            (Pawn|Components|CharacterMovement|SetMovementMode (Variables|Character|GetCharacterMovement) "MOVE_Falling" 0)))))))

(event Input|KeyboardEvents|S
  (params (Key :type Key%20Structure :default "None"))
  (bind _ledgeikhandle (Variables|Default|GetLedgeIKHandle))
  ;[1 1 1] Exiting the ledge
  (:Pressed
    (Variables|Default|SetIsOnLedge false)
    (Pawn|Components|CharacterMovement|SetMovementMode (Variables|Character|GetCharacterMovement) "MOVE_Falling" 0)
    (Variables|Default|SetbCanMove true)
    (Variables|Default|SetHandIKTargetAlpha 0.0)
    (Utilities|Time|ClearTimerbyFunctionName 0 "CheckIfLedgeHasSurface")
    (if (Utilities|Time|IsValidTimerHandle _ledgeikhandle)
      (Utilities|Time|ClearandInvalidateTimerbyHandle _ledgeikhandle))))

(fn ConstructionScript)

(fn TraceLedge
  (params (InitialZOffset :type Float%20%28double-precision%29) (TraceForward :type Float%20%28double-precision%29) (TraceVertical :type Float%20%28double-precision%29) (DrawDebugType :type EDrawDebugTrace%20Enum :default "None"))
  (bind _index (Utilities|FlowControl|ForLoopwithBreak 1 3 :!label _label)
    (:LoopBody
      (bind (_outhit _returnvalue) (Collision|SphereTraceByChannel (+ (Transformation|GetActorLocation) (Math|Vector|MakeVector 0.0 0.0 (+ InitialZOffset (* _index TraceVertical)))) (+ (+ (Transformation|GetActorLocation) (Math|Vector|MakeVector 0.0 0.0 (+ InitialZOffset (* _index TraceVertical)))) (* (Transformation|GetActorForwardVector) TraceForward)) 1e+01 "TraceTypeQuery1" false 0 DrawDebugType))
      (if _returnvalue
        (bind (_outhit_2 _returnvalue_2) (Collision|SphereTraceByChannel (+ (.ImpactPoint (Collision|BreakHitResult _outhit)) "0.000000,0.000000,20.000000") (.ImpactPoint (Collision|BreakHitResult _outhit)) 1e+01 "TraceTypeQuery1" false 0 DrawDebugType))
        (if (and _returnvalue_2 (not (.bInitialOverlap (Collision|BreakHitResult _outhit_2))))
          (Utilities|FlowControl|Sequence
            (:then_0
              (goto _label Break))
            (:then_1
              (return true (.ImpactPoint (Collision|BreakHitResult _outhit_2)) (.ImpactNormal (Collision|BreakHitResult _outhit))))))))
    (:Completed
      (return false "0, 0, 0" "0, 0, 0"))))

(fn FindLedgeHandIKLocation
  (params (Target :type Vector%20%28by%20ref%29) (RightOffset :type Float%20%28double-precision%29) (DrawDebugType :type EDrawDebugTrace%20Enum :default "None"))
  (bind _returnvalue (Transformation|GetActorForwardVector))
  (bind _returnvalue_2 (Transformation|GetActorRightVector))
  (bind _mesh (Variables|Character|GetMesh))
  (bind _capsulecomponent (Variables|Default|GetCapsuleComponent))
  (bind _returnvalue_3 (Transformation|GetWorldLocation _mesh))
  (bind _returnvalue_4 (Components|Capsule|GetScaledCapsuleHalfHeight _capsulecomponent))
  (bind _returnvalue_5 (* _returnvalue_2 RightOffset))
  (bind _returnvalue_6 (* _returnvalue 25.0))
  (bind _returnvalue_7 (+ _returnvalue_4 5e+01))
  (bind _returnvalue_8 (+ _returnvalue_3 (Math|Vector|MakeVector 0.0 0.0 _returnvalue_7)))
  (bind _returnvalue_9 (+ _returnvalue_8 _returnvalue_6 _returnvalue_5))
  (bind (_outhit _returnvalue_10) (Collision|SphereTraceByChannel _returnvalue_9 _returnvalue_9 15.0 "TraceTypeQuery1" false 0 DrawDebugType))
  (if _returnvalue_10
    (|SetBy-RefVar Target (.Location (Collision|BreakHitResult _outhit)))
    (return true)
    (else
      (return false))))
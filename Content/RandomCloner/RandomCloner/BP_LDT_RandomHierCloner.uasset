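; Construction-script cloner that scatters a random pick of static meshes over an XYZ grid as hierarchical instanced meshes.
; It creates one component per mesh, then adds instances with jittered position, rotation and uniform scale from seeded streams.
; Optional 90/180 yaw offsets use unseeded randomness, so they are not reproducible.
; Custom material and shadow settings go to randomly drawn components in each grid iteration, rather than explicitly to all.
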(event EventBeginPlay)

(event Collision|EventActorBeginOverlap
  (params (OtherActor :type Actor%20Object%20Reference)))

(event EventTick
  (params (DeltaSeconds :type Float%20%28single-precision%29)))

(fn ConstructionScript
  (bind _random_uniform_scale (Variables|Default|GetRandom%20Uniform%20Scale))
  (bind _random_rotation_y (Variables|Default|GetRandom%20Rotation%20Y))
  (bind _random_position_x (Variables|Default|GetRandom%20Position%20X))
  (bind _random_position_y (Variables|Default|GetRandom%20Position%20Y))
  (bind _random_position_z (Variables|Default|GetRandom%20Position%20Z))
  (bind _random_rotation_x (Variables|Default|GetRandom%20Rotation%20X))
  (bind _random_rotation_z (Variables|Default|GetRandom%20Rotation%20Z))
  (Variables|Default|SetSeed%20Cache%20Position%20X (Math|Random|MakeRandomStream (Variables|Default|GetSeed%20Position%20X)))
  (Variables|Default|SetSeed%20Cache%20Position%20Y (Math|Random|MakeRandomStream (Variables|Default|GetSeed%20Position%20Y)))
  (Variables|Default|SetSeed%20Cache%20Position%20Z (Math|Random|MakeRandomStream (Variables|Default|GetSeed%20Position%20Z)))
  (Variables|Default|SetSeed%20Cache%20Scale (Math|Random|MakeRandomStream (Variables|Default|GetSeed%20Scale%20)))
  (Variables|Default|SetSeed%20Cache%20Rotation%20Z (Math|Random|MakeRandomStream (Variables|Default|GetSeed%20Rotation%20Z)))
  (Variables|Default|SetSeed%20Random%20Pick%20Cache (Math|Random|MakeRandomStream (Variables|Default|GetSeed%20Random%20Pick)))
  (for _array_element (Variables|Default|GetStatic%20Mesh)
    (bind _returnvalue (AddComponent|AddHierarchicalInstancedStaticMeshComponent false))
    (Components|StaticMesh|SetStaticMesh _returnvalue _array_element)
    (Utilities|Array|Add (Variables|Default|GetComponents) _returnvalue))
  (for _index (range 0 (- (Variables|Default|GetZ%20Copy) 1))
    (for _index_2 (range 0 (- (Variables|Default|GetY%20Copy) 1))
      (for _index_3 (range 0 (- (Variables|Default|GetX%20Copy) 1))
        (switch Utilities|FlowControl|Switch|SwitchonRotationOption (Variables|Default|GetRandom%20Rotation%20Options)
          (:NewEnumerator2
            (Components|InstancedStaticMesh|AddInstance (.OutItem (Utilities|Array|RandomFromStream (Variables|Default|GetComponents) (Variables|Default|GetSeed%20Random%20Pick%20Cache))) (Math|Transform|MakeTransform (Math|Vector|MakeVector (+ (* _index_3 (Variables|Default|GetDistance%20X)) (Math|Random|RandomFloatinRangefromStream (Variables|Default|GetSeed%20Cache%20Position%20X) (* -1.0 _random_position_x) _random_position_x)) (+ (Math|Random|RandomFloatinRangefromStream (Variables|Default|GetSeed%20Cache%20Position%20Y) (* -1.0 _random_position_y) _random_position_y) (* _index_2 (Variables|Default|GetDistance%20Y))) (+ (* _index (Variables|Default|GetDistance%20Z)) (Math|Random|RandomFloatinRangefromStream (Variables|Default|GetSeed%20Cache%20Position%20Z) (* -1.0 _random_position_z) _random_position_z))) (Math|Rotator|MakeRotator (Math|Random|RandomFloatinRangefromStream (Variables|Default|GetSeed%20Cache%20Rotation%20Z) (* -1.0 _random_rotation_x) _random_rotation_x) (Math|Random|RandomFloatinRangefromStream (Variables|Default|GetSeed%20Cache%20Rotation%20Z) (* -1.0 _random_rotation_y) _random_rotation_y) (Math|Random|RandomFloatinRangefromStream (Variables|Default|GetSeed%20Cache%20Rotation%20Z) (* -1.0 _random_rotation_z) _random_rotation_z)) (+ (Math|Conversions|ToVector(Float) (Math|Random|RandomFloatinRangefromStream (Variables|Default|GetSeed%20Cache%20Scale) (* -1.0 _random_uniform_scale) _random_uniform_scale)) "1.000000,1.000000,1.000000")) false))
          (:NewEnumerator0
            (Components|InstancedStaticMesh|AddInstance (.OutItem (Utilities|Array|RandomFromStream (Variables|Default|GetComponents) (Variables|Default|GetSeed%20Random%20Pick%20Cache))) (Math|Transform|MakeTransform (Math|Vector|MakeVector (+ (* _index_3 (Variables|Default|GetDistance%20X)) (Math|Random|RandomFloatinRangefromStream (Variables|Default|GetSeed%20Cache%20Position%20X) (* -1.0 _random_position_x) _random_position_x)) (+ (Math|Random|RandomFloatinRangefromStream (Variables|Default|GetSeed%20Cache%20Position%20Y) (* -1.0 _random_position_y) _random_position_y) (* _index_2 (Variables|Default|GetDistance%20Y))) (+ (* _index (Variables|Default|GetDistance%20Z)) (Math|Random|RandomFloatinRangefromStream (Variables|Default|GetSeed%20Cache%20Position%20Z) (* -1.0 _random_position_z) _random_position_z))) (Math|Rotator|MakeRotator (Math|Random|RandomFloatinRangefromStream (Variables|Default|GetSeed%20Cache%20Rotation%20Z) (* -1.0 _random_rotation_x) _random_rotation_x) (Math|Random|RandomFloatinRangefromStream (Variables|Default|GetSeed%20Cache%20Rotation%20Z) (* -1.0 _random_rotation_y) _random_rotation_y) (+ (Math|Random|RandomFloatinRangefromStream (Variables|Default|GetSeed%20Cache%20Rotation%20Z) (* -1.0 _random_rotation_z) _random_rotation_z) (Utilities|Array|Get(acopy) (Variables|Default|GetRandom%2090) (Math|Random|RandomIntegerinRange 0 1)))) (+ (Math|Conversions|ToVector(Float) (Math|Random|RandomFloatinRangefromStream (Variables|Default|GetSeed%20Cache%20Scale) (* -1.0 _random_uniform_scale) _random_uniform_scale)) "1.000000,1.000000,1.000000")) false))
          (:NewEnumerator1
            (Components|InstancedStaticMesh|AddInstance (.OutItem (Utilities|Array|RandomFromStream (Variables|Default|GetComponents) (Variables|Default|GetSeed%20Random%20Pick%20Cache))) (Math|Transform|MakeTransform (Math|Vector|MakeVector (+ (* _index_3 (Variables|Default|GetDistance%20X)) (Math|Random|RandomFloatinRangefromStream (Variables|Default|GetSeed%20Cache%20Position%20X) (* -1.0 _random_position_x) _random_position_x)) (+ (Math|Random|RandomFloatinRangefromStream (Variables|Default|GetSeed%20Cache%20Position%20Y) (* -1.0 _random_position_y) _random_position_y) (* _index_2 (Variables|Default|GetDistance%20Y))) (+ (* _index (Variables|Default|GetDistance%20Z)) (Math|Random|RandomFloatinRangefromStream (Variables|Default|GetSeed%20Cache%20Position%20Z) (* -1.0 _random_position_z) _random_position_z))) (Math|Rotator|MakeRotator (Math|Random|RandomFloatinRangefromStream (Variables|Default|GetSeed%20Cache%20Rotation%20Z) (* -1.0 _random_rotation_x) _random_rotation_x) (Math|Random|RandomFloatinRangefromStream (Variables|Default|GetSeed%20Cache%20Rotation%20Z) (* -1.0 _random_rotation_y) _random_rotation_y) (+ (Utilities|Array|Get(acopy) (Variables|Default|GetRandom%20180) (Math|Random|RandomIntegerinRange 0 1)) (Math|Random|RandomFloatinRangefromStream (Variables|Default|GetSeed%20Cache%20Rotation%20Z) (* -1.0 _random_rotation_z) _random_rotation_z))) (+ (Math|Conversions|ToVector(Float) (Math|Random|RandomFloatinRangefromStream (Variables|Default|GetSeed%20Cache%20Scale) (* -1.0 _random_uniform_scale) _random_uniform_scale)) "1.000000,1.000000,1.000000")) false)))
        (if (Variables|Default|GetUse%20Custom%20Material?)
          (Rendering|Material|SetMaterial (.OutItem (Utilities|Array|RandomFromStream (Variables|Default|GetComponents) (Variables|Default|GetSeed%20Random%20Pick%20Cache))) 0 (Variables|Default|GetCustom%20Material)))
        (Rendering|SetCastShadow (.OutItem (Utilities|Array|RandomFromStream (Variables|Default|GetComponents) (Variables|Default|GetSeed%20Random%20Pick%20Cache))) (Variables|Optimization|GetCast%20Shadow))))))